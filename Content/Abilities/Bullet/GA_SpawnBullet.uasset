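; GA_SpawnBullet is a gameplay ability that fires a BP_Bullet from the ThirdPersonCharacter and handles its damage.
; On activation it commits, then spawns the bullet at the owner's location and rotation with that character as OwnerChara.
; It waits on two gameplay events at once: a hit applies GE_BulletDamage to the payload's target data and ends the ability.
; A bullet-destroy event ends it without damage.
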(event Ability|EventActivateAbility
  (bind _returnvalue (Ability|GetActorInfo))
  (Ability|CommitAbility)
  (bind _asthird_person_character (Utilities|Casting|CastToThirdPersonCharacter (.owneractor (Ability|GetActorInfo))))
  (Game|SpawnActorfromClass "/Game/Attack/BP_Bullet.BP_Bullet_C" (Math|Transform|MakeTransform (Transformation|GetActorLocation (.owneractor _returnvalue)) (Transformation|GetActorRotation (.owneractor _returnvalue))) "Undefined" 0 _asthird_person_character 0)
  (bind _payload (Ability|Tasks|WaitGameplayEvent "(TagName=\"Action.Attack.HitBullet\")" 0 true)
    (:then
      (Ability|Tasks|WaitGameplayEvent "(TagName=\"Ability.Action.DestryoBullet\")" 0 true
        (:EventReceived
          _)))
    (:EventReceived
      (GameplayEffects|ApplyGameplayEffectSpecToTarget (Ability|MakeOutgoingGameplayEffectSpec "/Game/Abilities/Bullet/GE_BulletDamage.GE_BulletDamage_C") (.TargetData (Utilities|Struct|BreakGameplayEventData _payload)))))
  (Ability|EndAbility))

(event Ability|EventOnEndAbility
  (params (bWasCancelled :type Boolean)))