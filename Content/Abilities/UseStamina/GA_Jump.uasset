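; Jump gameplay ability for the third-person character, which plays the AM_Jump montage and starts a stamina refresh afterwards.
; On activation it caches player 0's character, commits the ability and plays the montage, ending on any montage outcome.
; A failed commit does not call EndAbility.
; On end it applies GE_RefreshStamina to the owner and stores the effect handle on the character.
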(event Ability|EventActivateAbility
  (Utilities|IsValid (Variables|Default|GetCharacterRef)
    (:Is%20Valid
      _)
    (:Is%20Not%20Valid
      (bind _asthird_person_character (Utilities|Casting|CastToThirdPersonCharacter (Game|GetPlayerCharacter 0)))
      (Variables|Default|SetCharacterRef _asthird_person_character)))
  (Development|PrintString "Begin Jump")
  (bind _returnvalue (Ability|CommitAbility))
  (if _returnvalue
    (|PlayMontageandWaitProxy "None" "/Game/Mannequin/Animations/AM_Jump.AM_Jump" 1.0 "None" true 1.0
      (:OnCompleted
        _)
      (:OnBlendOut
        _)
      (:OnInterrupted
        _)
      (:OnCancelled
        _))
    (Ability|EndAbility)))

(event Ability|EventOnEndAbility
  (params (bWasCancelled :type Boolean))
  (Development|PrintString "End Jump")
  (bind _returnvalue (Ability|ApplyGameplayEffectToOwner "/Game/Abilities/Granted/GE_RefreshStamina.GE_RefreshStamina_C"))
  (Variables|/Game/ThirdPersonCPP/Blueprints/ThirdPersonCharacter.ThirdPersonCharacter_C|SetRefreshStaminaHandle (Variables|Default|GetCharacterRef) _returnvalue))